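; VR player pawn that handles view recentering and manual height adjustment through motion controller buttons.
; Right A resets HMD orientation and position, then rotates VROrigin by the negated world yaw of the camera.
; Left X and Y lower and raise VROrigin by DeltaAdjustmentOffset per press.
; All logic is input-driven, with no active BeginPlay or Tick behavior.
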(event EventBeginPlay
  (|CallParentFunction) ; This node is disabled and will not be called.\nDrag off pins to build functionality.
)

(event Collision|EventActorBeginOverlap
  (params (OtherActor :type Actor%20Object%20Reference)))

(event EventTick
  (params (DeltaSeconds :type Float%20%28single-precision%29))
  (|CallParentFunction DeltaSeconds) ; This node is disabled and will not be called.\nDrag off pins to build functionality.
)

(event Input|ActionEvents|InputActionRightStickA
  (params (Key :type Key%20Structure :default "None"))
  (:Pressed
    (Class|HeadMountedDisplayFunctionLibrary|ResetOrientationandPosition 0.0 "OrientationAndPosition")
    (Transformation|AddLocalRotation (Variables|Default|GetVROrigin) (Math|Rotator|MakeRotator 0.0 0.0 (* (.yaw (Transformation|GetWorldRotation (Variables|Default|GetCamera))) -1.0)) false false)))

(event Input|ActionEvents|InputActionLeftStickX
  (params (Key :type Key%20Structure :default "None"))
  (:Pressed
    (Transformation|AddLocalOffset (Variables|Default|GetVROrigin) (Math|Vector|MakeVector 0.0 0.0 (* (Variables|Default|GetDeltaAdjustmentOffset) -1.0)) false false)))

(event Input|ActionEvents|InputActionLeftStickY
  (params (Key :type Key%20Structure :default "None"))
  (:Pressed
    (Transformation|AddLocalOffset (Variables|Default|GetVROrigin) (Math|Vector|MakeVector 0.0 0.0 (Variables|Default|GetDeltaAdjustmentOffset)) false false)))

(fn ConstructionScript
  (|CallParentFunction))